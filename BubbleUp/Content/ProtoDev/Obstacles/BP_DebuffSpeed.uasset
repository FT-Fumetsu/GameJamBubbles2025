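; BP_DebuffSpeed is an obstacle volume that applies a movement debuff to the player's bubble character while it is inside.
; When the player pawn begins overlapping the Box, its BP_BubbleCharacter DeltaLocation is set to BubbleDeltaLocationDebuff.
; When the overlap ends, DeltaLocation is set to BubbleDeltaLocationBase rather than restoring the value it had on entry.
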(event `self.Box.OnComponentBeginOverlap`
  (params (OverlappedComponent :type "PrimitiveComponent Object Reference") (OtherActor :type "Actor Object Reference") (OtherComp :type "PrimitiveComponent Object Reference") (OtherBodyIndex :type Integer) (bFromSweep :type Boolean) (SweepResult :type "HitResult Structure (by ref)"))
  (if (== OtherActor (`GameplayStatics.GetPlayerPawn` 0))
    (bind _asbp_bubble_character (cast `/Game/ProtoDev/Character/BP_BubbleCharacter` OtherActor))
    (set `/Game/ProtoDev/Character/BP_BubbleCharacter.DeltaLocation` (`self.BubbleDeltaLocationDebuff`) _asbp_bubble_character)))

(event `self.Box.OnComponentEndOverlap`
  (params (OverlappedComponent :type "PrimitiveComponent Object Reference") (OtherActor :type "Actor Object Reference") (OtherComp :type "PrimitiveComponent Object Reference") (OtherBodyIndex :type Integer))
  (if (== OtherActor (`GameplayStatics.GetPlayerPawn` 0))
    (bind _asbp_bubble_character (cast `/Game/ProtoDev/Character/BP_BubbleCharacter` OtherActor))
    (set `/Game/ProtoDev/Character/BP_BubbleCharacter.DeltaLocation` (`self.BubbleDeltaLocationBase`) _asbp_bubble_character)))

(fn `UserConstructionScript`)