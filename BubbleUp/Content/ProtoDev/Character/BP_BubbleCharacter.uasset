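; Prototype player bubble character that drifts by a set offset every tick while the player steers it along the Y axis.
; BeginPlay adds the default Enhanced Input mapping context, and IA_Move applies sideways offsets, negated when InvertInputs is set.
; KillPlayer destroys the actor, shows the GameOver widget and prints an incremented DeathCount held on this Blueprint.
; Sphere overlap and hit events are empty, so nothing here triggers the death.
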(event `self.ReceiveBeginPlay`
  (bind _asplayer_controller (cast `PlayerController` (`GameplayStatics.GetPlayerController` 0)))
  (`EnhancedInputSubsystemInterface.AddMappingContext` (pcsubsystem `EnhancedInputLocalPlayerSubsystem` _asplayer_controller) "/Game/ThirdPerson/Input/IMC_Default.IMC_Default" 0 (struct)))

(event `EnhancedInput|/Game/ThirdPerson/Input/Actions/IA_Move`
  (params (ActionValue :type "Vector2D Structure") (ElapsedSeconds :type "Float (double-precision)") (TriggeredSeconds :type "Float (double-precision)") (InputAction :type "InputAction Object Reference" :default "/Game/ThirdPerson/Input/Actions/IA_Move.IA_Move"))
  (bind _returnvalue (* ActionValue_X 10.0))
  (:`Triggered`
    (if (`self.InvertInputs?`)
      (`self.K2_AddActorLocalOffset` (`KismetMathLibrary.MakeVector` 0.0 (* _returnvalue -1.0)))
      (else
        (`self.K2_AddActorLocalOffset` (`KismetMathLibrary.MakeVector` 0.0 _returnvalue))))))

(event `self.ReceiveTick`
  (params (DeltaSeconds :type "Float (single-precision)"))
  (`self.K2_AddActorLocalOffset` (`self.DeltaLocation`)))

(event `KillPlayer`
  (`self.K2_DestroyActor`)
  (`UserWidget.AddToViewport` (`self.GameOver`) 0)
  (bind _output_get (set `self.DeathCount` (+ (`self.DeathCount`) 1.0)))
  (`KismetSystemLibrary.PrintString` (`KismetStringLibrary.Conv_DoubleToString` _output_get)))

(event `self.Sphere1.OnComponentBeginOverlap`
  (params (OverlappedComponent :type "PrimitiveComponent Object Reference") (OtherActor :type "Actor Object Reference") (OtherComp :type "PrimitiveComponent Object Reference") (OtherBodyIndex :type Integer) (bFromSweep :type Boolean) (SweepResult :type "HitResult Structure (by ref)")))

(event `self.Sphere.OnComponentHit`
  (params (HitComponent :type "PrimitiveComponent Object Reference") (OtherActor :type "Actor Object Reference") (OtherComp :type "PrimitiveComponent Object Reference") (NormalImpulse :type "Vector Structure") (Hit :type "HitResult Structure (by ref)")))

(fn `UserConstructionScript`)